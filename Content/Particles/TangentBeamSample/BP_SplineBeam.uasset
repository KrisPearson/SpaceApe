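; Sample actor that draws a curved beam along its MainSplinePath spline using P_Beam Cascade emitters.
; On BeginPlay it spawns one emitter per spline segment, passing endpoint positions and tangents as Source and Target vector parameters, and prints each start tangent.
; Source positions and spawn locations use local space, while targets and tangents use world space.
; An unconnected chain would randomise a two-point spline first.
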(event EventBeginPlay
  (bind _mainsplinepath (Variables|Default|GetMainSplinePath))
  (for _index (range 0 (- (Spline|GetNumberOfSplinePoints _mainsplinepath) 2))
    (bind _returnvalue (Effects|SpawnEmitteratLocation "/Game/Particles/TangentBeamSample/P_Beam.P_Beam" (Spline|GetLocationatSplinePoint (Variables|Default|GetMainSplinePath) _index "Local")))
    (Effects|Components|ParticleSystem|SetVectorParameter _returnvalue "Source" (Spline|GetLocationatSplinePoint (Variables|Default|GetMainSplinePath) _index "Local"))
    (Effects|Components|ParticleSystem|SetVectorParameter _returnvalue "Source_Tan" (Spline|GetTangentatDistanceAlongSpline (Variables|Default|GetMainSplinePath) (Spline|GetDistanceAlongSplineatSplinePoint _mainsplinepath _index) "World"))
    (Effects|Components|ParticleSystem|SetVectorParameter _returnvalue "Target" (Spline|GetLocationatSplinePoint (Variables|Default|GetMainSplinePath) (+ _index 1) "World"))
    (Effects|Components|ParticleSystem|SetVectorParameter _returnvalue "Target_Tan" (Spline|GetTangentatDistanceAlongSpline (Variables|Default|GetMainSplinePath) (Spline|GetDistanceAlongSplineatSplinePoint _mainsplinepath (+ _index 1)) "World"))
    (Development|PrintString (Utilities|String|ToString(Vector) (Spline|GetTangentatDistanceAlongSpline (Variables|Default|GetMainSplinePath) (Spline|GetDistanceAlongSplineatSplinePoint _mainsplinepath _index) "World")))))

(event EventTick
  (params (DeltaSeconds :type Float%20%28single-precision%29)))

(fn ConstructionScript)