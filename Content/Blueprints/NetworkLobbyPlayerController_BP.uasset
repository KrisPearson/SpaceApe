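; Player controller for the network lobby that creates the lobby menu widget and relays lobby updates to it.
; On BeginPlay it builds and displays the menu, then registers it with the network game instance.
; Events forward player list and chat message updates to the menu, with a debug print for chat.
; A custom event opens a sign widget bound to the first actor found, and Escape quits the game.
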(event Custom|CustomEvent
  (params (PC :type Player%20Controller%20Object%20Reference))
  (bind _self self)
  ;[0 0 0] Comment
  (bind _outactors (Actor|GetAllActorsOfClass 0))
  (bind _returnvalue (UserInterface|CreateWidget "/Game/Items/Ui/NetworkSignWidget.NetworkSignWidget_C" _self (Utilities|Array|Get(acopy) _outactors) _self))
  (UserInterface|Viewport|AddtoViewport _returnvalue 0))

(event EventChatMessage
  (params (ChatMessage :type Text%20%28by%20ref%29))
  (Default|ReceiveChatMessage (Variables|Default|GetLobbyWidget) ChatMessage)
  (Development|PrintString "LobbyPC: EventReceiveChatMessage" true true "(R=0.992335,G=0.943905,B=1.000000,A=1.000000)" 5.0))

(event EventBeginPlay
  (bind _self self)
  (|CallParentFunction)
  (bind _asnetwork_game_instance_bp (Utilities|Casting|CastToNetworkGameInstance_BP (Game|GetGameInstance)))
  (bind _output_get (Variables|Default|SetNetworkGameInstanceRef _asnetwork_game_instance_bp))
  (bind _returnvalue (UserInterface|CreateWidget "/Game/UI/Lobby/LobbyMenu.LobbyMenu_C" _self _self _output_get))
  (bind _output_get_2 (Variables|Default|SetLobbyWidget _returnvalue))
  (UserInterface|Viewport|AddtoViewport _output_get_2 0)
  (Variables|/Game/TwinStickCPP/Game/NetworkGameInstance_BP.NetworkGameInstance_BP_C|SetLobbyMenuWidget _output_get _output_get_2))

(event EventUpdateUMGPlayerList
  (params (PlayerInfoArray :type Array%20of%20Lobby%20Player%20Info%20Structures))
  (Default|UpdatePlayerList (Variables|Default|GetLobbyWidget) PlayerInfoArray))

(event Input|KeyboardEvents|Escape
  (params (Key :type Key%20Structure :default "AnyKey"))
  ;[0 0 0] Comment
  (:Pressed
    (Game|QuitGame self "Quit")))

(fn ConstructionScript)